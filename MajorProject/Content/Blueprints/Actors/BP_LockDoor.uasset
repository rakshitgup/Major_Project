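; BP_LockDoor is an interactable door actor that stays locked until its key is picked up.
; PickUpKey sets a HasKey flag, and OnInteract prints a warning without it.
; With the key, each interaction toggles the closed state, playing or reversing a timeline that lerps the Pivot component's yaw to swing the door open or shut.
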(event EventBeginPlay
  (|CallParentFunction) ; This node is disabled and will not be called.\nDrag off pins to build functionality.
)

(event Collision|EventActorBeginOverlap
  (params (OtherActor :type Actor%20Object%20Reference))
  (|CallParentFunction OtherActor) ; This node is disabled and will not be called.\nDrag off pins to build functionality.
)

(event EventTick
  (params (DeltaSeconds :type Float%20%28single-precision%29))
  (|CallParentFunction DeltaSeconds) ; This node is disabled and will not be called.\nDrag off pins to build functionality.
)

(event EventOnInteract
  (params (Interacting%20Player :type Character%20Object%20Reference))
  (if (Variables|Default|GetHasKey?)
    (if (Variables|Default|GetisDoorClosed?)
      (Variables|Default|SetisDoorClosed? false)
      (bind _alpha (Timeline|OpenDoor Play)
        (:Update
          (Transformation|SetRelativeRotation (Variables|Default|GetPivot) (Math|Rotator|MakeRotator 0.0 0.0 (Math|Float|Lerp 0.0 -9e+01 _alpha)) false false)))
      (else
        (Variables|Default|SetisDoorClosed? true)
        (Timeline|OpenDoor Reverse)))
    (else
      (Development|PrintString "You need a key to open the door"))))

(event EventPickUpKey
  (Variables|Default|SetHasKey? true))

(fn ConstructionScript
  (|CallParentFunction))

(fn IsInteractable
  (return true))